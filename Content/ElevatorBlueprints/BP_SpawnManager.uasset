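; Spawn manager for the elevator level that builds a stack of floors on BeginPlay, then places the lift and the player.
; Floors are chained through each one's attach transform, using the last class in the Floors array, and each gets a call-lift button at its arrow marker.
; The lift and possessed first-person character get independent random heights in 500-unit steps, with horizontal positions taken from the last spawned floor.
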(event EventBeginPlay
  (bind _result (Math|Integer|DecrementInt (Math|Integer|Absolute(Integer) (Variables|Default|GetNumberOfFloors)))
    (:%20%20
      (for _index (range 0 _result)
        (CallFunction|CreateFloors))
      (CallFunction|SetLiftSpawnPosition)
      (CallFunction|SetPlayerSpawnPosition))))

(fn ConstructionScript)

(fn CreateFloors
  (bind _floors (Variables|Default|GetFloors))
  (bind _returnvalue (Game|SpawnActorfromClass (Utilities|Array|Get(acopy) _floors (Utilities|Array|LastIndex _floors)) (Variables|Default|GetNextSpawnPoint) "Undefined" "MultiplyWithRoot" 0 0))
  (bind _output_get (Variables|Default|SetFloor _returnvalue))
  (Game|SpawnActorfromClass "/Game/ElevatorBlueprints/BP_CallLiftButton.BP_CallLiftButton_C" (Transformation|GetWorldTransform (Variables|/Game/ElevatorBlueprints/BP_Floors.BP_Floors_C|GetArrow_Button _output_get)) "Undefined" "MultiplyWithRoot" 0 0)
  (bind _attachpoint (Default|GetAttachTransform _returnvalue))
  (Variables|Default|SetNextSpawnPoint _attachpoint))

(fn SetPlayerSpawnPosition
  (bind _floor (Variables|Default|GetFloor))
  (bind _arrow_player (Variables|/Game/ElevatorBlueprints/BP_Floors.BP_Floors_C|GetArrow_Player _floor))
  (bind _relativelocation (Variables|/Script/Engine.SceneComponent|GetRelativeLocation _arrow_player))
  (bind _asbp_first_person_character (Utilities|Casting|CastToBP_FirstPersonCharacter (Game|GetPlayerCharacter 0)))
  (Transformation|SetActorLocation _asbp_first_person_character (Math|Vector|MakeVector (.x _relativelocation) (.y _relativelocation) (* (Math|Random|RandomIntegerinRange 0 (Variables|Default|GetNumberOfFloors)) 500)) false false)
  (Pawn|Possess (Game|GetPlayerController 0) _asbp_first_person_character))

(fn SetLiftSpawnPosition
  (bind _floor (Variables|Default|GetFloor))
  (bind _rootcomponent (Variables|/Script/Engine.Actor|GetRootComponent _floor))
  (bind _returnvalue (Transformation|GetWorldLocation _rootcomponent))
  (Game|SpawnActorfromClass "/Game/ElevatorBlueprints/BP_Lift.BP_Lift_C" (Math|Transform|MakeTransform (Math|Vector|MakeVector (.x _returnvalue) (.y _returnvalue) (Math|Conversions|ToFloat(Integer) (* 500 (Math|Random|RandomIntegerinRange 0 (Variables|Default|GetNumberOfFloors))))) "0, 0, 0" "1.000000,1.000000,1.000000") "AdjustIfPossibleButAlwaysSpawn" "MultiplyWithRoot" 0 0))