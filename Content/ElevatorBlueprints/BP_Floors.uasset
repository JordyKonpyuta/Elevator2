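; BP_Floors is an elevator floor marker that tells a BP_Lift which floor it has reached.
; It derives its floor number by parsing the text after "Floors" in its own display name, so numbering depends on actor naming.
; When a lift overlaps its Box, it re-parses that number into the lift's CurrentFloor and prints debug messages.
; GetAttachTransform exposes the Arrow component's world transform as an attach point.
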(event OnComponentBeginOverlap(Box)
  (params (OverlappedComponent :type Primitive%20Component%20Object%20Reference) (OtherActor :type Actor%20Object%20Reference) (OtherComp :type Primitive%20Component%20Object%20Reference) (OtherBodyIndex :type Integer) (bFromSweep :type Boolean) (SweepResult :type Hit%20Result%20Structure%20%28by%20ref%29))
  (bind _asbp_lift (Utilities|Casting|CastToBP_Lift OtherActor)
    (:then
      (Development|PrintString "Hello")
      (bind _output_get (Variables|/Game/ElevatorBlueprints/BP_Lift.BP_Lift_C|SetCurrentFloor _asbp_lift (Math|Conversions|ToInteger(Byte) (.RightS (Utilities|String|Split (Utilities|GetDisplayName self) "Floors")))))
      (Development|PrintString (Utilities|String|ToString(Integer) _output_get)))
    (:CastFailed
      (Development|PrintString "Ouin"))))

(event EventBeginPlay
  (Variables|Default|SetFloorNumber (Math|Conversions|ToInteger(Byte) (.RightS (Utilities|String|Split (Utilities|GetDisplayName self) "Floors")))))

(fn ConstructionScript)

(fn GetAttachTransform
  (return (Transformation|GetWorldTransform (Variables|Default|GetArrow))))