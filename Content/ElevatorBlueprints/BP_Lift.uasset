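; Lift actor with sliding double doors and an on-screen control panel for travel between floors.
; MoveLift plays or reverses a timeline by target floor, setting lift height on finish from floor difference and fixed spacing.
; OpenDoors slides both doors apart via a timeline when stationary, reversing it while moving.
; A box trigger shows WBP_PanelControl to the first-person character, removing it and hiding the cursor on exit.
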(event OnComponentBeginOverlap(Box)
  (params (OverlappedComponent :type Primitive%20Component%20Object%20Reference) (OtherActor :type Actor%20Object%20Reference) (OtherComp :type Primitive%20Component%20Object%20Reference) (OtherBodyIndex :type Integer) (bFromSweep :type Boolean) (SweepResult :type Hit%20Result%20Structure%20%28by%20ref%29))
  ;[1 1 1] Create Panel Widget
  (Utilities|Casting|CastToBP_FirstPersonCharacter OtherActor)
  (bind _returnvalue (UserInterface|CreateWidget "/Game/ElevatorBlueprints/WBP_PanelControl.WBP_PanelControl_C"))
  (UserInterface|Viewport|AddtoViewport _returnvalue 0))

(event OnComponentEndOverlap(Box)
  (params (OverlappedComponent :type Primitive%20Component%20Object%20Reference) (OtherActor :type Actor%20Object%20Reference) (OtherComp :type Primitive%20Component%20Object%20Reference) (OtherBodyIndex :type Integer))
  ;[1 1 1] Create Panel Widget
  (Widget|RemovefromParent (stale OnComponentBeginOverlap(Box) _returnvalue))
  (Variables|/Script/Engine.PlayerController|SetbShowMouseCursor (Game|GetPlayerController 0) false))

(event Custom|MoveLift
  (params (IndexOfFloorToGo :type Integer))
  (bind _currentfloor (Variables|Default|GetCurrentFloor))
  ;[1 1 1] Lift Movement
  (Variables|Default|SetIsMoving? true)
  (if (> IndexOfFloorToGo (Variables|Default|GetCurrentFloor))
    (bind _up (Timeline|Timeline1 Play)
      (:Finished
        (Transformation|SetRelativeLocation (Variables|Default|GetLift) (Math|Vector|MakeVector 0.0 0.0 (Math|Float|Lerp (Math|Conversions|ToFloat(Integer) _currentfloor) (* (* _up 5e+02) (Math|Float|Absolute(Float) (- IndexOfFloorToGo _currentfloor))) _up)) false false)
        (if (== (Variables|Default|GetCurrentFloor) IndexOfFloorToGo)
          (Variables|Default|SetIsMoving? false))))
    (else
      (Timeline|Timeline1 Reverse))))

(event Custom|OpenDoors
  ;[1 1 1] Open/Close Doors
  (if (not (Variables|Default|GetIsMoving?))
    (bind _movement (Timeline|Timeline Play)
      (:Update
        (Transformation|SetRelativeLocation (Variables|Default|GetDoor_Left) (Math|Vector|MakeVector (* _movement -9e+01) 0.0 0.0) false false)
        (Transformation|SetRelativeLocation (Variables|Default|GetDoor_Right) (Math|Vector|MakeVector (* _movement 9e+01) 0.0 0.0) false false)))
    (else
      (Timeline|Timeline Reverse))))

(event EventBeginPlay
  (Utilities|Time|SetTimerbyEvent (EventDispatchers|CreateEvent :!event Custom|OpenDoors) 0.1))

(fn ConstructionScript)